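; BP_AIPatrolPoint is a patrol point that turns an arriving AI character to face the direction of its arrow component.
; On patroller entry it stores the character and opens a gate on Tick.
; While the gate is open, each tick interpolates the character's rotation toward the arrow's world rotation, and the patroller exit event closes the gate.
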(event `self.ReceiveTick`
  (params (DeltaSeconds :type "Float (single-precision)"))
  (`/Engine/EditorBlueprintResources/StandardMacros.Gate` true :!label _label
    (:`Exit`
      (`self.K2_SetActorRotation` (`self.Character`) (`KismetMathLibrary.RInterpTo` (`self.K2_GetActorRotation` (stale `OnPatrollerEntered` _output_get)) (`SceneComponent.K2_GetComponentRotation` (`self.Arrow`)) DeltaSeconds 2.0) false))))

(event `PatrollerExit`
  (goto _label :!via `Close`))

(event `OnPatrollerEntered`
  (params (Character :type "Character Object Reference"))
  (bind _output_get (set `self.Character` Character))
  (`|ExecutionSequence`
    (:`then_0`
      (goto _label :!via `Open`))))

(fn `UserConstructionScript`)