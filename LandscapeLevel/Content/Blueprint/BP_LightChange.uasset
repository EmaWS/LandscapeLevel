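; BP_LightChange is a trigger Blueprint that alters referenced lighting when its Trigger component is overlapped.
; The overlap event casts player 0's character to BP_ThirdPersonCharacter without checking the overlapping actor.
; On success, a sequence recolors every light in PointLightRef to Color, then hides the spot light component of each entry in SpotLightRef.
; Nothing in the graph reverts the change.
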(event `self.Trigger.OnComponentBeginOverlap`
  (params (OverlappedComponent :type "PrimitiveComponent Object Reference") (OtherActor :type "Actor Object Reference") (OtherComp :type "PrimitiveComponent Object Reference") (OtherBodyIndex :type Integer) (bFromSweep :type Boolean) (SweepResult :type "HitResult Structure (by ref)"))
  (cast `/Game/ThirdPerson/Blueprints/BP_ThirdPersonCharacter` (`GameplayStatics.GetPlayerCharacter` 0))
  (`|ExecutionSequence`
    (:`then_0`
      (for _array_element (`self.PointLightRef`)
        (`LightComponent.SetLightColor` (`Light.LightComponent` _array_element) (`KismetMathLibrary.Conv_ColorToLinearColor` (`self.Color`)) true)))
    (:`then_1`
      (for _array_element_2 (`self.SpotLightRef`)
        (`SceneComponent.SetVisibility` (`SpotLight.SpotLightComponent` _array_element_2) false false)))))

(fn `UserConstructionScript`)